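; ClickAndDrag_BP is an actor that rotates by click-and-drag mouse input, apparently as a camera orbit.
; Holding the left button past a short delay enables MouseX world yaw and MouseY local pitch, scaled by RotationSpeed.
; Presses and releases swap grab-hand cursors; Sphere collision starts off and is enabled on confirmed hold or release.
; Tick optionally clamps pitch between configurable limits, resetting roll when it does.
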(event Custom|Camera%20Limit
  (bind _returnvalue (Transformation|GetActorRotation))
  (bind _y_limit_min (Variables|Default|GetY%20Limit%20MIn))
  (bind _y_limit_max (Variables|Default|GetY%20Limit%20Max))
  (bind (_roll _pitch _yaw) (Math|Rotator|BreakRotator _returnvalue))
  (bind _returnvalue_2 (< _pitch _y_limit_min))
  ;[1 1 1] Camera Limit
  (if (Variables|Default|GetRotation%20Y%20Limit)
    (if (or _returnvalue_2 (> _pitch _y_limit_max))
      (Transformation|SetActorRotation (Math|Rotator|MakeRotator 0.0 (Math|Float|SelectFloat _y_limit_min _y_limit_max _returnvalue_2) _yaw)))))

(event EventBeginPlay
  ;[1 1 1] Collision STart
  (Collision|SetCollisionEnabled (Variables|Default|GetSphere) "NoCollision")
  (Variables|/Script/Engine.PlayerController|SetbShowMouseCursor (Game|GetPlayerController 0) true))

(event EventTick
  (params (DeltaSeconds :type Float%20%28single-precision%29))
  ;[1 1 1] Ticks
  (CallFunction|CameraLimit))

(event Input|MouseEvents|MouseX
  (params (AxisValue :type Float%20%28single-precision%29))
  ;[1 1 1] Camera Rotation
  (if (Variables|Default|GetHold)
    (Class|Actor|AddActorWorldRotation (Math|Rotator|MakeRotator 0.0 0.0 (* (* AxisValue (Variables|Default|GetRotationSpeed)) -1.0)))))

(event Input|MouseEvents|MouseY
  (params (AxisValue :type Float%20%28single-precision%29))
  ;[1 1 1] Camera Rotation
  (if (Variables|Default|GetHold)
    (Transformation|AddActorLocalRotation (Math|Rotator|MakeRotator 0.0 (* (* AxisValue (Variables|Default|GetRotationSpeed)) -1.0) 0.0) false false)))

(event Input|MouseEvents|LeftMouseButton
  (params (Key :type Key%20Structure :default "None"))
  (bind _returnvalue (Game|GetPlayerController 0))
  ;[1 1 1] Camera Rotation
  (:Pressed
    (Variables|/Script/Engine.PlayerController|SetCurrentMouseCursor _returnvalue "GrabHandClosed")
    (Utilities|FlowControl|Delay 0.15)
    (if (Game|Player|IsInputKeyDown _returnvalue Key)
      (Variables|Default|SetHold true)
      (Collision|SetCollisionEnabled (Variables|Default|GetSphere) "QueryAndPhysics")))
  (:Released
    (Variables|/Script/Engine.PlayerController|SetCurrentMouseCursor _returnvalue "GrabHand")
    (Variables|Default|SetHold false)
    (Collision|SetCollisionEnabled (Variables|Default|GetSphere) "QueryAndPhysics")))

(fn ConstructionScript)